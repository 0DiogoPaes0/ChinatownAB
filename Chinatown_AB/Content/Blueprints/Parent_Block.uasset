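; Parent block actor for a destructible structure hit by birds, with a Wood, Stone or Glass BlockType.
; The construction script sets the material from BlockType.
; Damage is truncated and subtracted from that type's health; at zero the block plays a sound, spawns a break particle and destroys itself.
; Overlap by a "Bird"-tagged actor swaps Wood and Stone to cracked materials, independently of health, while Glass has no cracked look.
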(event OnComponentBeginOverlap(BlockCollision)
  (params (OverlappedComponent :type Primitive%20Component%20Object%20Reference) (OtherActor :type Actor%20Object%20Reference) (OtherComp :type Primitive%20Component%20Object%20Reference) (OtherBodyIndex :type Integer) (bFromSweep :type Boolean) (SweepResult :type Hit%20Result%20Structure%20%28by%20ref%29))
  (if (Actor|ActorHasTag OtherActor "Bird")
    (switch Utilities|FlowControl|Switch|SwitchonBlockType (Variables|Default|GetBlockType)
      (:NewEnumerator0
        (Rendering|Material|SetMaterial (Variables|Default|GetStaticMesh) 0 "/Game/Assets/Mat/StylizedWood_Broken_Mat.StylizedWood_Broken_Mat"))
      (:NewEnumerator1
        (Rendering|Material|SetMaterial (Variables|Default|GetStaticMesh) 0 "/Game/Assets/Mat/CrackedStoneStylized.CrackedStoneStylized")))))

(event Game|Damage|EventAnyDamage
  (params (Damage :type Float%20%28single-precision%29) (DamageType :type Damage%20Type%20Object%20Reference) (InstigatedBy :type Controller%20Object%20Reference) (DamageCauser :type Actor%20Object%20Reference))
  (Variables|Default|SetDamage (Math|Float|Truncate Damage))
  (switch Utilities|FlowControl|Switch|SwitchonBlockType (Variables|Default|GetBlockType)
    (:NewEnumerator0
      (CallFunction|SetWoodHealth))
    (:NewEnumerator1
      (CallFunction|SetStoneHealth))
    (:NewEnumerator2
      (CallFunction|SetGlassHealth))))

(fn ConstructionScript
  (switch Utilities|FlowControl|Switch|SwitchonBlockType (Variables|Default|GetBlockType)
    (:NewEnumerator0
      (Rendering|Material|SetMaterial (Variables|Default|GetStaticMesh) 0 "/Game/Assets/Mat/StylizedWood_Mat.StylizedWood_Mat"))
    (:NewEnumerator1
      (Rendering|Material|SetMaterial (Variables|Default|GetStaticMesh) 0 "/Game/Assets/Mat/StoneStylized.StoneStylized"))
    (:NewEnumerator2
      (Rendering|Material|SetMaterial (Variables|Default|GetStaticMesh) 0 "/Game/Assets/Mat/Glass.Glass"))))

(fn SetWoodHealth
  (Variables|Default|SetWood%20Health (- (Variables|Default|GetWood%20Health) (Variables|Default|GetDamage)))
  (if (<= (Variables|Default|GetWood%20Health) 0)
    (Audio|PlaySound2D "/Game/Sounds/SFX/Funny_Rubber_Balloon_Deflate_5.Funny_Rubber_Balloon_Deflate_5" 1.0 1.0 0.0 0 0)
    (Effects|SpawnEmitteratLocation "/Game/InfinityBladeEffects/Effects/FX_Breakables/barrel/P_BarrelBreak_Wood.P_BarrelBreak_Wood" (Transformation|GetWorldLocation (Variables|Default|GetBlockPhysics)) "0, 0, 0" "0.200000,0.200000,0.200000")
    (Actor|DestroyActor)))

(fn SetGlassHealth
  (Variables|Default|SetGlass%20Health (- (Variables|Default|GetGlass%20Health) (Variables|Default|GetDamage)))
  (if (<= (Variables|Default|GetGlass%20Health) 0)
    (Audio|PlaySound2D "/Game/Sounds/SFX/Glass_Break_Cue.Glass_Break_Cue" 1.0 1.0 0.0 0 0)
    (Effects|SpawnEmitteratLocation "/Game/InfinityBladeEffects/Effects/FX_Breakables/pot/P_PotBreak_Ceramic.P_PotBreak_Ceramic" (Transformation|GetWorldLocation (Variables|Default|GetBlockPhysics)))
    (Actor|DestroyActor)))

(fn SetStoneHealth
  (Variables|Default|SetStone%20Health (- (Variables|Default|GetStone%20Health) (Variables|Default|GetDamage)))
  (if (<= (Variables|Default|GetStone%20Health) 0)
    (Audio|PlaySound2D "/Game/Sounds/SFX/Stone_Break_Cue.Stone_Break_Cue" 1.0 1.0 0.0 0 0)
    (Effects|SpawnEmitteratLocation "/Game/InfinityBladeEffects/Effects/FX_Breakables/pot/P_PotBreak_Ceramic.P_PotBreak_Ceramic" (Transformation|GetWorldLocation (Variables|Default|GetBlockPhysics)))
    (Actor|DestroyActor)))
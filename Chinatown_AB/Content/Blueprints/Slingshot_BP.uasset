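; Slingshot pawn for an Angry Birds-style game that launches Red_BP birds by touch drag and handles camera zoom and pan.
; Drag offset sets the impulse, previewed each tick by spawning Dot_BP actors along a predicted projectile path.
; Release applies the impulse to the physics-enabled bird, then spawns a replacement after a delay.
; AddPigs counts toward the level's tagged pig total and prints a win message.
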(event Custom|Action%20Mapping
  ;[0.15 0.15 0.15 0.5] Action Mapping
  (bind _asplayer_controller (Utilities|Casting|CastToPlayerController (Pawn|GetController)))
  (Utilities|IsValid (PlayerController|LocalPlayerSubsystems|GetEnhancedInputLocalPlayerSubsystem _asplayer_controller)
    (:Is%20Valid
      (Input|AddMappingContext (PlayerController|LocalPlayerSubsystems|GetEnhancedInputLocalPlayerSubsystem _asplayer_controller) "/Game/ThirdPerson/Input/IMC_Default.IMC_Default" 0 "(bIgnoreAllPressedKeysUntilRelease=True,bForceImmediately=False,bNotifyUserSettings=False)"))))

(event Custom|Add%20Pigs
  (bind _output_get (Variables|Default|SetPigs (+ (stale _output_get) 1)))
  (if (>= (Variables|Default|GetPigs) (Variables|Default|GetMax%20Pigs))
    (Development|PrintString "You Won")))

(event Input|EnhancedActionEvents|EnhancedInputActionIA_ZoomIn
  (params (ActionValue :type Vector%202D%20Structure) (ElapsedSeconds :type Float%20%28double-precision%29) (TriggeredSeconds :type Float%20%28double-precision%29) (InputAction :type Input%20Action%20Object%20Reference :default "/Game/ThirdPerson/Input/Actions/IA_ZoomIn.IA_ZoomIn"))
  (bind _springarm (Variables|Default|GetSpringArm))
  (Variables|/Script/Engine.SpringArmComponent|SetTargetArmLength _springarm (Math|Float|Clamp(Float) (- (Variables|/Script/Engine.SpringArmComponent|GetTargetArmLength _springarm) 5e+01) 1e+03 2.5e+03)))

(event Input|EnhancedActionEvents|EnhancedInputActionIA_ZoomOut
  (params (ActionValue :type Vector%202D%20Structure) (ElapsedSeconds :type Float%20%28double-precision%29) (TriggeredSeconds :type Float%20%28double-precision%29) (InputAction :type Input%20Action%20Object%20Reference :default "/Game/ThirdPerson/Input/Actions/IA_ZoomOut.IA_ZoomOut"))
  (bind _springarm (Variables|Default|GetSpringArm))
  (Variables|/Script/Engine.SpringArmComponent|SetTargetArmLength _springarm (Math|Float|Clamp(Float) (+ (Variables|/Script/Engine.SpringArmComponent|GetTargetArmLength _springarm) 5e+01) 1e+03 2.5e+03)))

(event Input|EnhancedActionEvents|EnhancedInputActionIA_Pan_Left
  (params (ActionValue :type Vector%202D%20Structure) (ElapsedSeconds :type Float%20%28double-precision%29) (TriggeredSeconds :type Float%20%28double-precision%29) (InputAction :type Input%20Action%20Object%20Reference :default "/Game/ThirdPerson/Input/Actions/IA_Pan_Left.IA_Pan_Left"))
  (bind _springarm (Variables|Default|GetSpringArm))
  (Variables|/Script/Engine.SpringArmComponent|SetSocketOffset _springarm (Math|Vector|MakeVector 0.0 (Math|Float|Clamp(Float) (- (.y (Variables|/Script/Engine.SpringArmComponent|GetSocketOffset _springarm)) 5e+01) -8e+02 1e+03) 0.0)))

(event Input|EnhancedActionEvents|EnhancedInputActionIA_Pan_Right
  (params (ActionValue :type Vector%202D%20Structure) (ElapsedSeconds :type Float%20%28double-precision%29) (TriggeredSeconds :type Float%20%28double-precision%29) (InputAction :type Input%20Action%20Object%20Reference :default "/Game/ThirdPerson/Input/Actions/IA_Pan_Right.IA_Pan_Right"))
  (bind _springarm (Variables|Default|GetSpringArm))
  (Variables|/Script/Engine.SpringArmComponent|SetSocketOffset _springarm (Math|Vector|MakeVector 0.0 (Math|Float|Clamp(Float) (- (.y (Variables|/Script/Engine.SpringArmComponent|GetSocketOffset _springarm)) -5e+01) -8e+02 1e+03) 0.0)))

(event EventBeginPlay
  (CallFunction|ActionMapping)
  (Variables|/Script/Engine.PlayerController|SetbShowMouseCursor (Game|GetPlayerController 0) true)
  (bind _returnvalue (Game|SpawnActorfromClass "/Game/Blueprints/Red_BP.Red_BP_C" (Math|Transform|MakeTransform (Transformation|GetWorldLocation (Variables|Default|GetLaunch%20Position)) "0, 0, 0" "1.000000,1.000000,1.000000") "Undefined" "MultiplyWithRoot" 0 0))
  (bind _output_get (Variables|Default|SetRed%20BP _returnvalue))
  (Physics|SetSimulatePhysics (Variables|/Game/Blueprints/Red_BP.Red_BP_C|GetRed_Physics _output_get) false)
  (bind _outactors (Actor|GetAllActorswithTag "Pig"))
  (Variables|Default|SetMax%20Pigs (Utilities|Array|Length _outactors)))

(event EventTick
  (params (DeltaSeconds :type Float%20%28single-precision%29))
  (if (Variables|Default|GetShouldPredict?)
    (bind _returnvalue (Class|WidgetLayoutLibrary|GetMousePositiononPlatform))
    (Variables|Default|SetImpulse%20Z (* (.y (- _returnvalue (Variables|Default|GetClick%20Original%20Pos))) 3.0))
    (Variables|Default|SetImpulse%20Y (* (.x (- _returnvalue (Variables|Default|GetClick%20Original%20Pos))) 4.0))
    (bind _outpathpositions (Class|GameplayStatics|BlueprintPredictProjectilePathbyTraceChannel (Transformation|GetWorldLocation (Variables|Default|GetLaunch%20Position)) (Math|Vector|MakeVector 0.0 (* (.x (- _returnvalue (Variables|Default|GetClick%20Original%20Pos))) 4.0) (* (.y (- _returnvalue (Variables|Default|GetClick%20Original%20Pos))) 3.0)) true 2.0 "ECC_WorldDynamic" false 0 "None" 0.1 1e+01 1.0))
    (for _array_element _outpathpositions
      (Game|SpawnActorfromClass "/Game/Blueprints/Dot_BP.Dot_BP_C" (Math|Transform|MakeTransform _array_element "0, 0, 0" "1.000000,1.000000,1.000000") "Undefined" "MultiplyWithRoot" 0 0))))

(event Input|TouchEvents|InputTouch
  (params (Location :type Vector) (FingerIndex :type ETouchIndex%20Enum))
  ;[0.15 0.15 0.15 0.5] Input Touch
  (:Pressed
    (if (Variables|Default|GetCan%20Shoot?)
      (Variables|Default|SetShouldPredict? true)
      (bind _returnvalue (Class|WidgetLayoutLibrary|GetMousePositiononPlatform))
      (Variables|Default|SetClick%20Original%20Pos _returnvalue)
      (if (Variables|Default|GetAuto%20Zoom?)
        _)))
  (:Released
    (Variables|Default|SetShouldPredict? false)
    (Physics|SetSimulatePhysics (Variables|/Game/Blueprints/Red_BP.Red_BP_C|GetRed_Physics (Variables|Default|GetRed%20BP)) true)
    (Physics|AddImpulse (Variables|/Game/Blueprints/Red_BP.Red_BP_C|GetRed_Physics (Variables|Default|GetRed%20BP)) (Math|Vector|MakeVector 0.0 (Variables|Default|GetImpulse%20Y) (Variables|Default|GetImpulse%20Z)) "None" true)
    (Audio|PlaySound2D "/Game/Sounds/SFX/14155_cartoon_bird_argue_furious-full.14155_cartoon_bird_argue_furious-full" 1.0 1.0 0.0 0 0)
    (Variables|Default|SetCan%20Shoot? false)
    (Utilities|FlowControl|Delay 1.0)
    (bind _returnvalue_2 (Game|SpawnActorfromClass "/Game/Blueprints/Red_BP.Red_BP_C" (Math|Transform|MakeTransform (Transformation|GetWorldLocation (Variables|Default|GetLaunch%20Position)) "0, 0, 0" "1.000000,1.000000,1.000000") "Undefined" "MultiplyWithRoot" 0 0))
    (bind _output_get (Variables|Default|SetRed%20BP _returnvalue_2))
    (Physics|SetSimulatePhysics (Variables|/Game/Blueprints/Red_BP.Red_BP_C|GetRed_Physics _output_get) false)
    (Variables|Default|SetCan%20Shoot? true)))

(fn ConstructionScript)
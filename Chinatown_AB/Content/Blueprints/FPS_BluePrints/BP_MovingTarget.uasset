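; BP_MovingTarget is an FPS target actor that moves back and forth until it is hit.
; A looping timer flips its Direction every TimeToChange, while Tick offsets it along the normalized Direction by Speed without delta-time scaling or sweep.
; OnHit spawns an emitter and plays an explosion sound at the root's location, then destroys the actor.
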(event Custom|CustomEvent
  (Variables|Default|SetDirection (* (Variables|Default|GetDirection) -1.0)))

(event Custom|OnHit
  (bind _defaultsceneroot (Variables|Default|GetDefaultSceneRoot))
  (bind _returnvalue (Transformation|GetWorldLocation _defaultsceneroot))
  (Effects|SpawnEmitteratLocation 0 _returnvalue)
  (Audio|PlaySoundatLocation "/Game/StarterContent/Audio/Explosion02.Explosion02" _returnvalue "0, 0, 0" 1.0 1.0 0.0 0 0 0 0)
  (Actor|DestroyActor))

(event EventTick
  (params (DeltaSeconds :type Float%20%28single-precision%29))
  (Transformation|AddActorWorldOffset (* (Math|Vector|Normalize (Variables|Default|GetDirection)) (Variables|Default|GetSpeed))))

(event EventBeginPlay
  (Utilities|Time|SetTimerbyEvent (delegate Custom|CustomEvent) (Variables|Default|GetTime%20To%20Change) true))

(fn ConstructionScript)
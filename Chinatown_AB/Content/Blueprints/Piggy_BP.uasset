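; Piggy_BP is a destructible pig target in what appears to be a slingshot game.
; On BeginPlay it waits a random delay, plays an oink sound, caches the Slingshot_BP actor and rolls a random health value.
; AnyDamage subtracts truncated damage; at zero health it plays a death sound, spawns a wood-break particle at its physics component, calls AddPigs on the slingshot and destroys itself.
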(event EventBeginPlay
  (Utilities|FlowControl|Delay (Math|Random|RandomFloatinRange 1.0 5.0))
  (Audio|PlaySound2D "/Game/Sounds/SFX/13995_cartoon_pig_yes.13995_cartoon_pig_yes" 1.0 1.0 0.0 0 0)
  (bind _returnvalue (Actor|GetActorOfClass "/Game/Blueprints/Slingshot_BP.Slingshot_BP_C"))
  (Variables|Default|SetAs%20Slingshot%20BP _returnvalue)
  (Variables|Default|SetPig%20Health (Math|Random|RandomIntegerinRange 50 60)))

(event Game|Damage|EventAnyDamage
  (params (Damage :type Float%20%28single-precision%29) (DamageType :type Damage%20Type%20Object%20Reference) (InstigatedBy :type Controller%20Object%20Reference) (DamageCauser :type Actor%20Object%20Reference))
  (Variables|Default|SetPig%20Health (- (Variables|Default|GetPig%20Health) (Math|Float|Truncate Damage)))
  (if (<= (Variables|Default|GetPig%20Health) 0)
    (Audio|PlaySound2D "/Game/Sounds/SFX/Pig_JBA04_54_1.Pig_JBA04_54_1" 1.0 1.0 0.0 0 0)
    (Effects|SpawnEmitteratLocation "/Game/InfinityBladeEffects/Effects/FX_Breakables/Box/P_BoxBreak_Wood.P_BoxBreak_Wood" (Transformation|GetWorldLocation (Variables|Default|GetPiggy_Physics)))
    (Default|AddPigs (Variables|Default|GetAs%20Slingshot%20BP))
    (Actor|DestroyActor)))

(fn ConstructionScript)
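; Red_BP is a physics-based actor, likely the Red bird projectile, that damages what it hits and then removes itself.
; The first overlap on Red_Collision passes a DoOnce and applies random damage to the other actor, with no filtering.
; After a random delay it plays a sound, spawns a wood-break emitter at RedPhysics and destroys itself.
; A "Block" tag check exists but is disconnected and never runs.
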(event OnComponentBeginOverlap(Red_Collision)
  (params (OverlappedComponent :type Primitive%20Component%20Object%20Reference) (OtherActor :type Actor%20Object%20Reference) (OtherComp :type Primitive%20Component%20Object%20Reference) (OtherBodyIndex :type Integer) (bFromSweep :type Boolean) (SweepResult :type Hit%20Result%20Structure%20%28by%20ref%29))
  (Utilities|FlowControl|DoOnce false
    (:Completed
      (Game|Damage|ApplyDamage OtherActor (Math|Random|RandomFloatinRange 4e+01 6e+01) 0 0)
      (Utilities|FlowControl|Delay (Math|Random|RandomFloatinRange 4.0 1e+01))
      (Audio|PlaySound2D 0 1.0 1.0 0.0 0 0)
      (Effects|SpawnEmitteratLocation "/Game/InfinityBladeEffects/Effects/FX_Breakables/barrel/P_BarrelBreak_Wood.P_BarrelBreak_Wood" (Transformation|GetWorldLocation (Variables|Default|GetRed_Physics)))
      (Actor|DestroyActor))))

(fn ConstructionScript)